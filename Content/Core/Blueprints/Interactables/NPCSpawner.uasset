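; NPC spawner interactable that periodically spawns AI pawns while it is active.
; Tick calls UpdateSpawner, which uses a DoOnce gate followed by a Delay and reset to spawn at a set frequency.
; Each spawn creates the configured pawn class with the BHConsumer behavior tree at the Spawnpoint component, ignoring collision failures.
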(event `self.ReceiveTick`
  (params (DeltaSeconds :type "Float (single-precision)"))
  (`self.UpdateSpawner`))

(event `UpdateSpawner`
  ; Spawn NPC with some delay
  (if (`self.IsActive`)
    (`/Engine/EditorBlueprintResources/StandardMacros.DoOnce` false :!label _label
      (:`Completed`
        (`AIBlueprintHelperLibrary.SpawnAIFromClass` (`self.PawnClassToSpawn`) "/Game/Core/AI/BehaviorTrees/BHConsumer.BHConsumer" (`SceneComponent.K2_GetComponentLocation` (`self.Spawnpoint`)) (struct) true null)
        (`KismetSystemLibrary.Delay` (`self.SpawnFrequency`))
        (goto _label :!via `Reset`)))))

(fn `UserConstructionScript`)