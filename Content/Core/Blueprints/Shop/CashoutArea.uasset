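; Shop checkout area actor that queues NPC consumers and cashes them out one at a time.
; Tick polls the queue, and a DoOnce gate starts each cashout by moving everyone to evenly spaced points from the cashier.
; The front NPC's items drop randomly in the unload area, then after a delay its blackboard flags it to exit.
; The items are destroyed and the NPC is dequeued, resetting the gate.
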(event `self.ReceiveTick`
  (params (DeltaSeconds :type "Float (single-precision)"))
  (`self.UpdateQueue`))

(event `AddConsumerToQueue`
  (params (Consumer :type "/Game/Core/AI/Consumer Object Reference"))
  (`KismetArrayLibrary.Array_AddUnique` (`self.ConsumersQueue`) Consumer))

(event `UpdateQueue`
  (bind _consumersqueue (`self.ConsumersQueue`))
  (bind (_origin _boxextent) (`KismetSystemLibrary.GetComponentBounds` (`self.ItemsUnloadArea`)))
  (bind _output (`|GetArrayItem` _consumersqueue))
  (bind _pickeditems (`/Game/Core/AI/Consumer.PickedItems` _output))
  ; Update queue
  ;; Check if there is any NPC to process
  (if (> (`KismetMathLibrary.Conv_IntToBool` (`KismetArrayLibrary.Array_Length` _consumersqueue)) 0)
    ;; Proceed only one NPC at once
    (`/Engine/EditorBlueprintResources/StandardMacros.DoOnce` false :!label _label
      (:`Completed`
        (`|ExecutionSequence`
          (:`then_0`
            ;; Force to move each NPC in the queue close to the cashier calculating new positions
            (for (_array_element _array_index) _consumersqueue
              (bind _point (`self.CalculateQueuePointForSpecieficPosition` _array_index))
              (`AITask_MoveTo.AIMoveTo` (`AIBlueprintHelperLibrary.GetAIController` _array_element) _point null (`self.AcceptanceRadiusToCashier`) "Disable" "Enable" true true true "Enable" "Disable")))
          (:`then_1`
            ;; Drop all the items held by NPC to speciefied unload zone
            (for _array_element_2 _pickeditems
              (`/Game/Core/Blueprints/Shop/Items/1ItemMain.Drop` _array_element_2 (`KismetMathLibrary.RandomPointInBoundingBox` _origin (/ _boxextent 2.0))))
            ;; Simulate cashout routine
            (`KismetSystemLibrary.Delay` (`self.ProceedingDelay`))
            ;; Let NPC go to the exit by setting IsOnTheWayToExit blackboard variable
            (`BlackboardComponent.SetValueAsBool` (`AIBlueprintHelperLibrary.GetBlackboard` (`AIBlueprintHelperLibrary.GetAIController` _output)) (`self.OnTheWayToExitBBParameterName`) true)
            ;; Destroy cashied items - don't need them anymore
            (for _array_element_3 _pickeditems
              (`self.K2_DestroyActor` _array_element_3))
            (`KismetSystemLibrary.PrintString` "Consumer is cashed out")
            ;; Remove NPC from the queue and unlock process for next one
            (`KismetArrayLibrary.Array_RemoveItem` _consumersqueue _output)
            (goto _label :!via `Reset`)))))))

(fn `CalculateQueuePoint`
  (returns (Point :type "Vector Structure"))
  (return (+ (`SceneComponent.K2_GetComponentLocation` (`self.ConsumerPoint`)) (* (`self.StandingQueueVector`) (* (`self.StandingQueueStep`) (`KismetArrayLibrary.Array_Length` (`self.ConsumersQueue`)))))))

(fn `CalculateQueuePointForSpecieficPosition`
  (params (Number :type Integer))
  (returns (Point :type "Vector Structure"))
  (return (+ (`SceneComponent.K2_GetComponentLocation` (`self.ConsumerPoint`)) (* (`self.StandingQueueVector`) (* (`self.StandingQueueStep`) Number)))))

(fn `UserConstructionScript`)