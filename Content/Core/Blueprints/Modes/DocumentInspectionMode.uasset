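; Gameplay ability that runs the document inspection mode, where a valid or fake ID is presented for comparison against a set of entries.
; On activation it shows the inspection widget with UI-only input, fills its entries, and adds a GameManager-generated document with a 50% chance of being fake.
; On end it restores game input, removes the widgets and has GameManager regenerate the valid ID database.
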(event `self.K2_ActivateAbility`
  (bind _returnvalue (`GameplayStatics.GetPlayerController` 0))
  ; Start inspection mode: create inspection widget, fill it with entries, create document to compare
  (set `PlayerController.bShowMouseCursor` true _returnvalue)
  (bind _returnvalue_2 (`|CreateWidget` "/Game/Core/Widgets/IDSInspectionWidget.IDSInspectionWidget_C" _returnvalue))
  (`/Game/Core/Widgets/IDSInspectionWidget.FillWidgetWithEntries` _returnvalue_2)
  (set `self.InspectionWidget` _returnvalue_2)
  (`WidgetBlueprintLibrary.SetInputMode_UIOnlyEx` _returnvalue _returnvalue_2)
  (`UserWidget.AddToViewport` _returnvalue_2 0)
  (bind _asgame_manager (cast `/Game/Core/GameManager` (`GameplayStatics.GetGameInstance`)))
  ;; Randomly with 50% chance assign invalid document
  (if (`KismetMathLibrary.RandomBool`)
    ; Generate and add invalid document
    (bind _invalidentry (`/Game/Core/GameManager.GenerateInvalidIDEntry` _asgame_manager))
    (`/Game/Core/Widgets/IDSInspectionWidget.AddDocumentToCompare` _returnvalue_2 _invalidentry true)
    (else
      ; Generate and add valid document
      (bind _validentry (`/Game/Core/GameManager.GenerateValidIDEntry` _asgame_manager))
      (`/Game/Core/Widgets/IDSInspectionWidget.AddDocumentToCompare` _returnvalue_2 _validentry false))))

(event `self.K2_OnEndAbility`
  (params (bWasCancelled :type Boolean))
  (bind _returnvalue (`GameplayStatics.GetPlayerController` 0))
  (bind _inspectionwidget (`self.InspectionWidget`))
  ; Reset mode, destroy all related widgets and regenerate database on inspection end
  (`WidgetBlueprintLibrary.SetInputMode_GameOnly` _returnvalue)
  (set `PlayerController.bShowMouseCursor` false _returnvalue)
  (`/Game/Core/Widgets/IDSInspectionWidget.DestroyAllInstancedWidgets` _inspectionwidget)
  (`Widget.RemoveFromParent` _inspectionwidget)
  (bind _asgame_manager (cast `/Game/Core/GameManager` (`GameplayStatics.GetGameInstance`)))
  (`/Game/Core/GameManager.GenerateValidIDSDatabase` _asgame_manager))