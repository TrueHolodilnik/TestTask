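; Utility function collection with shared helpers for date display, food category lookups and player input toggling.
; DateTimeToText builds a zero-padded DD.MM.YYYY text, while two map lookups translate a food category into its material or class.
; SwitchInputAvailability enables or disables input on the first player's character, branching on IsMoveInputIgnored, a flag it reads but never sets.
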(fn `DateTimeToText`
  (params (DateTime :type "DateTime Structure"))
  (returns (OutText :type Text))
  ; Converts DateTime struct to DD.MM.YYYY format
  (return (`KismetTextLibrary.Conv_StringToText` (`KismetStringLibrary.Concat_StrStr` (`KismetStringLibrary.Concat_StrStr` (`KismetMathLibrary.SelectString` "0" "" (< DateTime_Day 10)) (`KismetStringLibrary.Conv_IntToString` DateTime_Day)) "." (`KismetStringLibrary.Concat_StrStr` (`KismetMathLibrary.SelectString` "0" "" (< DateTime_Month 10)) (`KismetStringLibrary.Conv_IntToString` DateTime_Month)) "." (`KismetStringLibrary.Conv_IntToString` DateTime_Year)))))

(fn `FoodCategoryToClass`
  (params (FoodCategory :type "/Game/Core/Enums/FoodCategories Enum" :default "NewEnumerator0"))
  (returns (ClassOutput :type "/Game/Core/Blueprints/Shop/Items/1ItemMain Class Reference"))
  (locals (FoodCategoryToClass :type "Map of /Game/Core/Enums/FoodCategories Enum to /Game/Core/Blueprints/Shop/Items/1ItemMain Class Reference"))
  (return (`BlueprintMapLibrary.Map_Find` (`local.FoodCategoryToClass`) FoodCategory)))

(fn `FoodCategoryToMaterial`
  (params (FoodCategory :type "/Game/Core/Enums/FoodCategories Enum" :default "NewEnumerator0"))
  (returns (MaterialOut :type "Material Object Reference"))
  (locals (FoodCategoriesToMaterialMap :type "Map of /Game/Core/Enums/FoodCategories Enum to Material Object Reference"))
  (return (`BlueprintMapLibrary.Map_Find` (`local.FoodCategoriesToMaterialMap`) FoodCategory)))

(fn `SwitchInputAvailability`
  (bind _returnvalue (`GameplayStatics.GetPlayerCharacter` null))
  (bind _returnvalue_2 (`GameplayStatics.GetPlayerController` null))
  (if (`Controller.IsMoveInputIgnored` _returnvalue_2)
    (`Actor.EnableInput` _returnvalue _returnvalue_2)
    (else
      (`Actor.DisableInput` _returnvalue _returnvalue_2))))