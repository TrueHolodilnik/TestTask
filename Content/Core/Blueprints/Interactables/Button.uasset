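; Interactable button Blueprint that switches a linked interactable on and off along with itself.
; Its activate and deactivate events each call the parent implementation, forward the same call to InteractableToActivate, then print a debug message.
; The link is used without a validity check, and the construction script only calls the parent.
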(event `self.ActivateInteractable`
  ; Activation logic: pressing the button it activates itself and the linked interactable
  (`parent.ActivateInteractable`)
  (`self.ActivateInteractable` (`self.InteractableToActivate`))
  (`KismetSystemLibrary.PrintString` "Button activated"))

(event `self.DeactivateInteractable`
  ; Activation logic: pressing the button it activates itself and the linked interactable
  (`parent.DeactivateInteractable`)
  (`self.DeactivateInteractable` (`self.InteractableToActivate`))
  (`KismetSystemLibrary.PrintString` "Button deactivated"))

(fn `UserConstructionScript`
  (`parent.UserConstructionScript`))